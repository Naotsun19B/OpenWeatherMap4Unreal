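; Test actor that exercises a WeatherMap accessor by requesting Tokyo's weather in Celsius on BeginPlay.
; It binds data and error events, printing the received time, city and weather or the HTTP response code.
; On success it also passes the weather icon URL to an on-screen W_TestWidget, which is removed on EndPlay.
; Both handlers then unbind the accessor's events; unconnected nodes showcase its API, including requests by city ID and coordinates.
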(event `self.ReceiveBeginPlay`
  (`|ExecutionSequence`
    (:`then_0`
      (bind _returnvalue (`|CreateWidget` "/Game/W_TestWidget.W_TestWidget_C"))
      (bind _output_get (set `self.IconWidget` _returnvalue))
      (`UserWidget.AddToViewport` _output_get 0))
    (:`then_1`
      (bind _weathermapaccessor (`OpenWeatherMap4UnrealBPLibrary.CreateWeatherMapAccessor` (`self.API_Key`)))
      (bind _output_get_2 (set `self.WeatherMap` _weathermapaccessor))
      (`WeatherMapAccessor.RequestWeatherMapDataWithCityName` _output_get_2 "Tokyo" "TU_Celsius")
      (`|ExecutionSequence`
        (:`then_0`
          (add `WeatherMapAccessor.OnReceivedWeatherMapData` (`self.WeatherMap`) (delegate `OnReceivedWeatherMapData`)))
        (:`then_1`
          (add `WeatherMapAccessor.OnRecivedErrorCode` (`self.WeatherMap`) (delegate `OnRecievedErrorCode`)))))))

(event `OnReceivedWeatherMapData`
  (bind _weathermap (`self.WeatherMap`))
  (bind (_citydata _weatherdata _updatedtime _returnvalue) (`WeatherMapAccessor.GetReceivedWeatherMapData` (`self.WeatherMap`)))
  (if _returnvalue
    (set `self.CityData` _citydata)
    (set `self.WeatherData` _weatherdata)
    (set `self.UpdatedTime` _updatedtime)
    (`|ExecutionSequence`
      (:`then_0`
        (`KismetSystemLibrary.PrintString` (`OpenWeatherMap4UnrealBPLibrary.ConvertDateTimeToString` (`self.UpdatedTime`)) true true (struct :`G` 1.0 :`A` 1.0) 10.0)
        (`KismetSystemLibrary.PrintString` (`OpenWeatherMap4UnrealBPLibrary.ConvertCityDataToString` (`self.CityData`)) true true (struct :`G` 1.0 :`A` 1.0) 10.0)
        (`KismetSystemLibrary.PrintString` (`OpenWeatherMap4UnrealBPLibrary.ConvertWeatherDataToString` (`self.WeatherData`)) true true (struct :`G` 1.0 :`A` 1.0) 10.0))
      (:`then_1`
        (bind (_url _returnvalue_2) (`WeatherMapAccessor.GetWeatherIconURL` (`self.WeatherMap`)))
        (if _returnvalue_2
          (`/Game/W_TestWidget.ChangeIcon` (`self.IconWidget`) _url)))
      (:`then_2`
        (clear `WeatherMapAccessor.OnReceivedWeatherMapData` _weathermap :!label _label)
        (clear `WeatherMapAccessor.OnFailureCommunication` _weathermap)))))

(event `self.ReceiveEndPlay`
  (params (EndPlayReason :type "EEndPlayReason Enum" :default "Destroyed"))
  (`Widget.RemoveFromParent` (`self.IconWidget`)))

(event `OnRecievedErrorCode`
  (bind _responsecode (`WeatherMapAccessor.GetReceivedHttpStatesCode` (`self.WeatherMap`)))
  (`KismetSystemLibrary.PrintString` (`KismetStringLibrary.Conv_IntToString` _responsecode) true false (struct :`R` 1.0 :`A` 1.0) 5.0)
  (goto _label))

(fn `UserConstructionScript`)